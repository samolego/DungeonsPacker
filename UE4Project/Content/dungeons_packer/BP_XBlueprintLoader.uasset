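; Loader actor that, on BeginPlay, spawns prefab actors from a PNG in dungeons_packer named after its outer's outer, then destroys itself.
; The image is copied to a render target for pixel reads, with each row encoding one actor in four RGBA pixels.
; Byte pairs give the Prefabs table index and position, while bit-packed 10-bit triples give rotation and scale, with position and rotation offset by the loader's transform.
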(event `self.ReceiveBeginPlay`
  (bind _textrender (`self.TextRender`))
  (bind (_rendertarget _sizey) (`self.readImage` (`KismetStringLibrary.Concat_StrStr` (`KismetSystemLibrary.GetProjectContentDirectory`) "dungeons_packer/" (`KismetSystemLibrary.GetObjectName` (`KismetSystemLibrary.GetOuterObject` (`KismetSystemLibrary.GetOuterObject` self))) ".png")))
  (for _index (range _sizey)
    (bind _returnvalue (`KismetRenderingLibrary.ReadRenderTargetRawPixel` _rendertarget 0 _index))
    (bind _returnvalue_2 (`KismetRenderingLibrary.ReadRenderTargetRawPixel` _rendertarget 1 _index))
    (bind _returnvalue_3 (`KismetRenderingLibrary.ReadRenderTargetRawPixel` _rendertarget 2 _index))
    (bind (_r _g _b _a) (break `LinearColor` _returnvalue_3))
    (bind _rotation (`self.getRotation` _r _g _b _a))
    (bind _returnvalue_4 (`KismetRenderingLibrary.ReadRenderTargetRawPixel` _rendertarget 3 _index))
    (bind (_r_2 _g_2 _b_2 _a_2) (break `LinearColor` _returnvalue_4))
    (bind (_x _y _z) (`self.getEncodedFloats` _r_2 _g_2 _b_2 _a_2))
    (bind (_r_3 _g_3 _b_3 _a_3) (break `LinearColor` _returnvalue))
    (bind _actorclass (`self.getPrefabClass` (`self.decodeCoordinate` _r_3 _g_3)))
    (bind (_r_4 _g_4 _b_4 _a_4) (break `LinearColor` _returnvalue_2))
    (bind _returnvalue_5 (/ (`KismetMathLibrary.MakeVector` _x _y _z) 100.0))
    (`|SpawnActorFromClass` _actorclass (`KismetMathLibrary.MakeTransform` (+ (`KismetMathLibrary.GreaterGreater_VectorRotator` (* (`KismetMathLibrary.MakeVector` (`KismetMathLibrary.Conv_IntToDouble` (`self.decodeCoordinate` _r_4 _g_4)) (`KismetMathLibrary.Conv_IntToDouble` (`self.decodeCoordinate` _b_4 _a_4)) (`KismetMathLibrary.Conv_IntToDouble` (`self.decodeCoordinate` _b_3 _a_3))) 10) (`self.K2_GetActorRotation` self)) (`self.K2_GetActorLocation` self)) _rotation _returnvalue_5) "AlwaysSpawn" "OverrideRootScale" (`self.GetOwner` self) (`self.GetInstigator` self))
    (`TextRenderComponent.SetWorldSize` _textrender 200.0)
    (bind _returnvalue_6 (`GameplayStatics.GetCurrentLevelName` true))
    (`TextRenderComponent.K2_SetText` _textrender (`KismetTextLibrary.Conv_StringToText` (`KismetStringLibrary.Concat_StrStr` " classnmae: " (`KismetSystemLibrary.Conv_SoftClassReferenceToString` (`|ConvertAsset` _actorclass)) " level name " _returnvalue_6 "pixel data: " (`KismetStringLibrary.Conv_VectorToString` _returnvalue_5)))))
  (`self.K2_DestroyActor`))

(fn `decodeCoordinate`
  (params (highByte :type "Float (double-precision)") (lowByte :type "Float (double-precision)"))
  (returns (decoded :type Integer))
  (return (+ (* (`KismetMathLibrary.Round` highByte) 256) (`KismetMathLibrary.Round` lowByte))))

(fn `getEncodedFloats`
  (params (R :type "Float (double-precision)") (G :type "Float (double-precision)") (B :type "Float (double-precision)") (A :type "Float (double-precision)"))
  (returns (x :type "Float (double-precision)") (y :type "Float (double-precision)") (z :type "Float (double-precision)"))
  (bind _returnvalue (`KismetMathLibrary.Round` G))
  (bind _returnvalue_2 (`KismetMathLibrary.Round` B))
  (return (`KismetMathLibrary.Conv_IntToDouble` (`KismetMathLibrary.Or_IntInt` (* (`KismetMathLibrary.And_IntInt` (`KismetMathLibrary.Round` R) 255) 4) (/ (`KismetMathLibrary.And_IntInt` _returnvalue 192) 64))) (`KismetMathLibrary.Conv_IntToDouble` (`KismetMathLibrary.Or_IntInt` (* (`KismetMathLibrary.And_IntInt` _returnvalue 63) 16) (/ (`KismetMathLibrary.And_IntInt` _returnvalue_2 240) 16))) (`KismetMathLibrary.Conv_IntToDouble` (`KismetMathLibrary.Or_IntInt` (* (`KismetMathLibrary.And_IntInt` _returnvalue_2 15) 64) (`KismetMathLibrary.And_IntInt` (/ (`KismetMathLibrary.Round` A) 4) 63)))))

(fn `getPrefabClass`
  (params (index :type Integer))
  (returns (actorClass :type "Actor Class Reference"))
  (bind _returnvalue (`|GetDataTableRow` "/Game/dungeons_packer/prefabs.prefabs" (`KismetStringLibrary.Conv_StringToName` (`KismetStringLibrary.Conv_IntToString` index)))
    (:`then`
      (return (`|ConvertAsset` (`.BP_ClassPath_8_AB7242DC44A130CE381B4296862EA4AA` (break `/Game/dungeons_packer/S_ActorLibrary` _returnvalue)))))))

(fn `getRotation`
  (params (r :type "Float (double-precision)") (g :type "Float (double-precision)") (b :type "Float (double-precision)") (a :type "Float (double-precision)"))
  (returns (rotation :type "Rotator Structure"))
  (bind (_x _y _z) (`self.getEncodedFloats` r g b a))
  (return (`KismetMathLibrary.MakeRotator` (+ _x (.roll (`self.K2_GetActorRotation` self))) (+ _y (.pitch (`self.K2_GetActorRotation` self))) (+ _z (.yaw (`self.K2_GetActorRotation` self))))))

(fn `readImage`
  (params (Filename :type String))
  (returns (renderTarget :type "TextureRenderTarget2D Object Reference") (sizeY :type Integer))
  (bind _returnvalue (`KismetRenderingLibrary.ImportFileAsTexture2D` Filename))
  (set `Texture.SRGB` false _returnvalue)
  (bind _returnvalue_2 (`Texture2D.Blueprint_GetSizeX` _returnvalue))
  (bind _returnvalue_3 (`Texture2D.Blueprint_GetSizeY` _returnvalue))
  (bind _returnvalue_4 (`KismetRenderingLibrary.CreateRenderTarget2D` _returnvalue_2 _returnvalue_3 "RTF_RGBA8"))
  (bind (_canvas _size _context) (`KismetRenderingLibrary.BeginDrawCanvasToRenderTarget` _returnvalue_4))
  (`Canvas.K2_DrawTexture` _canvas _returnvalue (0.0 0.0) (`KismetMathLibrary.MakeVector2D` (`KismetMathLibrary.Conv_IntToDouble` _returnvalue_2) (`KismetMathLibrary.Conv_IntToDouble` _returnvalue_3)) (0.0 0.0) (1.0 1.0) (struct :`R` 1.0 :`G` 1.0 :`B` 1.0 :`A` 1.0) "BLEND_Opaque" 0.0 (0.5 0.5))
  (`KismetRenderingLibrary.EndDrawCanvasToRenderTarget` _context)
  (return _returnvalue_4 _returnvalue_3))

(fn `UserConstructionScript`)